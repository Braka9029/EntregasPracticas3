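; BP_Puerta is a two-leaf door that slides apart when an interacting actor holds a key.
; The Interactuar event checks TieneLlave and prints an angry face if the key is missing.
; A timeline adds its two track values to each leaf's current relative X every update, so movement accumulates.
; The Abierta guard sets itself to false, so it never blocks another play.
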(event EventBeginPlay)

(event Collision|EventActorBeginOverlap
  (params (OtherActor :type Actor%20Object%20Reference)))

(event EventTick
  (params (DeltaSeconds :type Float%20%28single-precision%29)))

(event EventInteractuar
  (params (Actor :type BP%20Third%20Person%20Character%20Object%20Reference))
  (bind _hojaderecha (Variables|Default|GetHojaDerecha))
  (bind _hojaizqueirda (Variables|Default|GetHojaIzqueirda))
  (if (Variables|/Game/ThirdPerson/Blueprints/BP_ThirdPersonCharacter.BP_ThirdPersonCharacter_C|GetbTieneLlave Actor)
    (if (not (Variables|Default|GetbAbierta))
      (Variables|Default|SetbAbierta false)
      (bind (_direction _hizquierda _derecha) (Timeline|Timeline Play)
        (:Update
          (Transformation|SetRelativeLocation _hojaderecha (Math|Vector|MakeVector (+ (.x (Variables|/Script/Engine.SceneComponent|GetRelativeLocation _hojaderecha)) _derecha) 0.0 0.0) false false)
          (Transformation|SetRelativeLocation _hojaizqueirda (Math|Vector|MakeVector (+ _hizquierda (.x (Variables|/Script/Engine.SceneComponent|GetRelativeLocation _hojaizqueirda))) 0.0 0.0) false false))))
    (else
      (Development|PrintString ">:("))))

(fn ConstructionScript)